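; GameModeBP is a game mode Blueprint that periodically spawns an actor while the player pawn's move input is ignored.
; A timer starts at SpawnTime and counts down every Tick by world delta seconds.
; When it is below zero and the GGJ20Pawn ignores move input, it spawns the actor and resets the timer.
; The spawn location is the pawn's scaled forward vector, without adding the pawn's position.
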(event `self.ReceiveBeginPlay`
  (set `self.CurrentTime` (`self.SpawnTime`)))

(event `self.ReceiveTick`
  (params (DeltaSeconds :type "Float (single-precision)"))
  (bind _returnvalue (`GameplayStatics.GetPlayerPawn` 0))
  (set `self.CurrentTime` (- (`self.CurrentTime`) (`GameplayStatics.GetWorldDeltaSeconds`)))
  (bind _asggj20pawn (cast `GGJ20Pawn` _returnvalue))
  (if (and (`Pawn.IsMoveInputIgnored` _asggj20pawn) (< (`self.CurrentTime`) 0.0))
    (`|SpawnActorFromClass` "/Game/CPPBluprint/EnemyProtoBP.EnemyProtoBP_C" (`KismetMathLibrary.MakeTransform` (* (`self.GetActorForwardVector` _returnvalue) 20.0)) "Undefined" "OverrideRootScale" null null)
    (set `self.CurrentTime` (`self.SpawnTime`))))

(fn `UserConstructionScript`)