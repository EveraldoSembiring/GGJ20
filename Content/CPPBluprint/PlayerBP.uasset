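; Player actor that flies toward the mouse cursor, with health shown as actor scale and a color passed to the fairy animation Blueprint.
; Tick turns and sweeps it toward the cursor hit point at constant height, stopping when close.
; Health changes rescale it and start a frame-counted IFrame timer, during which an active pushback replaces steering until the count reaches zero.
; Color is set to white on BeginPlay; random color cycling is disconnected.
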(event `self.ReceiveBeginPlay`
  (`self.UpdateScale`)
  (`self.ChangeColor` (make `Color` 255 255 255 255)))

(event `self.ReceiveTick`
  (params (DeltaSeconds :type "Float (single-precision)"))
  (bind (_returnvalue_x _returnvalue_y _returnvalue_z) (`KismetMathLibrary.BreakVector` (`self.K2_GetActorLocation`)))
  (bind _hitresult (`PlayerController.GetHitResultUnderCursorByChannel` (`GameplayStatics.GetPlayerController` 0) "TraceTypeQuery1" true))
  (bind _returnvalue (`KismetMathLibrary.MakeVector` (.x (`.Location` (`GameplayStatics.BreakHitResult` _hitresult))) (.y (`.Location` (`GameplayStatics.BreakHitResult` _hitresult))) _returnvalue_z))
  (`|ExecutionSequence`
    (:`then_0`
      ;[1 1 1] Comment
      (if (`self.OnPushBack`)
        _
        (elif (> (`KismetMathLibrary.Vector_Distance` (`self.K2_GetActorLocation`) _returnvalue) 70.0)
          (`self.K2_SetActorLocationAndRotation` (+ (`self.K2_GetActorLocation`) (* (`self.GetActorForwardVector`) (* (`self.ForwardSpeed`) DeltaSeconds))) (`KismetMathLibrary.RLerp` (`self.K2_GetActorRotation`) (`KismetMathLibrary.FindLookAtRotation` (`self.K2_GetActorLocation`) _returnvalue) (* DeltaSeconds (`self.RotateSpeed`)) true) true))))
    (:`then_1`
      (if (> (`self.IFrame`) 0)
        (if (`self.OnPushBack`)
          (`self.K2_SetActorLocation` (+ (`self.K2_GetActorLocation`) (* (`self.GetActorForwardVector`) (* (`self.PushBackSpeed`) DeltaSeconds))) true))
        (bind _result (`/Engine/EditorBlueprintResources/StandardMacros.DecrementInt` (`self.IFrame`))
          (:`  `
            (if (== _result 0)
              (set `self.OnPushBack` false))))))))

(fn `ChangeColor`
  (params (NewColor :type "Color Structure"))
  (bind _output_get (set `self.Color` NewColor))
  (bind _asfiary_animation_blueprint (cast `/Game/TwinStickBP/Fiary/FiaryAnimationBlueprint` (`SkeletalMeshComponent.GetAnimInstance` (`self.SkeletalMesh`))))
  (`/Game/TwinStickBP/Fiary/FiaryAnimationBlueprint.Evolution` _asfiary_animation_blueprint _output_get))

(fn `HealthGain`
  (params (Enemy :type "/Game/CPPBluprint/Enemy Object Reference"))
  (bind _result (`/Engine/EditorBlueprintResources/StandardMacros.IncrementInt` (`self.Health`))
    (:`  `
      (set `self.Health` (`KismetMathLibrary.Clamp` _result 0 (`self.MaxHealth`)))
      (`self.UpdateScale`)
      (`self.SetToIFrame` 12))))

(fn `HealthLost`
  (params (Enemy :type "/Game/CPPBluprint/Enemy Object Reference"))
  (bind _result (`/Engine/EditorBlueprintResources/StandardMacros.DecrementInt` (`self.Health`))
    (:`  `
      (set `self.Health` (`KismetMathLibrary.Clamp` _result 0 (`self.MaxHealth`)))
      (`self.UpdateScale`)
      (`self.SetToIFrame` 90))))

(fn `PushBack`
  (set `self.OnPushBack` true))

(fn `SetToIFrame`
  (params (iFrame :type Integer))
  (set `self.IFrame` iFrame))

(fn `UpdateScale`
  (`self.SetActorScale3D` (* (`KismetMathLibrary.Vector_One`) (`KismetMathLibrary.FClamp` (/ (`KismetMathLibrary.Conv_IntToDouble` (`self.Health`)) (`KismetMathLibrary.Conv_IntToDouble` (`self.MaxHealth`))) 0.3 1.0))))

(fn `UserConstructionScript`)